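; BP_CombatDrone is a combat drone Blueprint with key-driven weapon test controls.
; Keys 1 and 2 fire the rocket and defensive weapon mounts through their reload-timed fire function.
; Key 3 runs a debug-drawn visibility line trace along the drone's forward vector and prints to screen.
; BeginPlay, Tick, overlap and the construction script are empty.
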(event `self.ReceiveBeginPlay`)

(event `Key|One`
  (params (Key :type "Key Structure"))
  (:`Pressed`
    (`SimWeaponMountComponent.FireMountedWeaponWithReloadTime` (`self.WeaponMount_Rocket`))))

(event `Key|Two`
  (params (Key :type "Key Structure"))
  (:`Pressed`
    (`SimWeaponMountComponent.FireMountedWeaponWithReloadTime` (`self.WeaponMount_Defensive`))))

(event `Key|Three`
  (params (Key :type "Key Structure"))
  (bind _returnvalue (`self.K2_GetActorLocation`))
  (:`Pressed`
    (`KismetSystemLibrary.LineTraceSingle` :`Start` _returnvalue :`End` (+ _returnvalue (* (`self.GetActorForwardVector`) (5000.0 5000.0 5000.0))) :`TraceChannel` "TraceTypeQuery1" :`DrawDebugType` "ForDuration")
    (`KismetSystemLibrary.PrintString` "HitActor")))

(fn `UserConstructionScript`)